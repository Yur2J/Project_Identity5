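; Game mode that assigns each joining player a Hunter or Survivor character.
; BeginPlay casts the first player character to Hunter, then to Survivor only if that succeeds, storing the results as references.
; PostLogin takes the class from one stored reference, spawns it at a random PlayerStart and has the player possess it.
; HunterSpawned selects Hunter when true, Survivor otherwise, and is never set here.
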(event `self.ReceiveBeginPlay`
  (bind _returnvalue (`GameplayStatics.GetPlayerCharacter` 0))
  (bind _asbp_hunter (cast `/Game/Blueprints/BP_Hunter` _returnvalue))
  (set `self.HunterCharacterClass` _asbp_hunter)
  (bind _asbp_survivor (cast `/Game/Blueprints/BP_Survivor` _returnvalue))
  (set `self.SurvivorCharacterClass` _asbp_survivor))

(event `self.K2_PostLogin`
  (params (NewPlayer :type "PlayerController Object Reference"))
  (bind _outactors (`GameplayStatics.GetAllActorsOfClass` "/Script/Engine.PlayerStart"))
  (if (`self.HunterSpawned`)
    (bind _returnvalue_location (`KismetMathLibrary.BreakTransform` (`self.GetTransform` (`KismetArrayLibrary.Array_Random` _outactors))))
    (bind _returnvalue (`|SpawnActorFromClass` (`GameplayStatics.GetObjectClass` (`self.HunterCharacterClass`)) (`KismetMathLibrary.MakeTransform` _returnvalue_location) "Undefined" "MultiplyWithRoot" null null))
    (`Controller.Possess` NewPlayer _returnvalue)
    (else
      (bind _returnvalue_2 (`|SpawnActorFromClass` (`GameplayStatics.GetObjectClass` (`self.SurvivorCharacterClass`)) (`KismetMathLibrary.MakeTransform` _returnvalue_location) "Undefined" "MultiplyWithRoot" null null))
      (`Controller.Possess` NewPlayer _returnvalue_2))))

(fn `UserConstructionScript`)