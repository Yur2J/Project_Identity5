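; Lobby game mode that gives each joining player a hunter or survivor pawn.
; On PostLogin it reads SelectedRole from BP_PlayerState, then spawns and possesses the matching BP_Hunter or BP_Survivor, with no spawn transform set.
; Disconnected, unused logic remains for HunterSpawned-based assignment at random PlayerStarts, and for showing a waiting widget and server-traveling to InGame at two players.
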(event `self.K2_PostLogin`
  (params (NewPlayer :type "PlayerController Object Reference"))
  (bind _asbp_player_state (cast `/Game/Blueprints/Lobby/BP_PlayerState` (`Controller.PlayerState` NewPlayer)))
  (`|ExecutionSequence`
    (:`then_0`
      (bind _selectedrole (`/Game/Blueprints/Lobby/BP_PlayerState.SelectedRole` _asbp_player_state))
      (if (`|EnumEquality` _selectedrole "NewEnumerator1")
        (bind _returnvalue (`|SpawnActorFromClass` "/Game/Blueprints/Lobby/InGame/Character/BP_Hunter.BP_Hunter_C" (`KismetMathLibrary.MakeTransform` (0.0 0.0 0.0)) "Undefined" "MultiplyWithRoot" null null))
        (`Controller.Possess` NewPlayer _returnvalue)))
    (:`then_1`
      (if (`|EnumEquality` _selectedrole "NewEnumerator2")
        (bind _returnvalue_2 (`|SpawnActorFromClass` "/Game/Blueprints/Lobby/InGame/Character/BP_Survivor.BP_Survivor_C" (`KismetMathLibrary.MakeTransform` (0.0 0.0 0.0)) "Undefined" "MultiplyWithRoot" null null))
        (`Controller.Possess` NewPlayer _returnvalue_2)))))

(fn `UserConstructionScript`)