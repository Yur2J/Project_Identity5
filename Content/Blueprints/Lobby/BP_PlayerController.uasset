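; Lobby player controller that handles the Hunter or Survivor role pick.
; On BeginPlay the local controller caches the game state, adds the default input mapping and opens the role-select widget in UI-only mode.
; C2S_SelectedRole, gated on a local controller, checks and sets the game state's taken flags, then writes the role to the player state.
; S2C-named events show the lobby and waiting widgets.
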(event `self.ReceiveBeginPlay`
  (bind _returnvalue (`GameplayStatics.GetPlayerController` 0))
  (if (`self.IsLocalController`)
    (`|ExecutionSequence`
      (:`then_0`
        (bind _asbp_game_state (cast `/Game/Blueprints/Lobby/BP_GameState` (`GameplayStatics.GetGameState`))
          (:`then`
            (set `self.GameStateRef` _asbp_game_state)
            (if (`self.IsLocalPlayerController`)
              (`EnhancedInputSubsystemInterface.AddMappingContext` (subsystem `EnhancedInputLocalPlayerSubsystem`) "/Game/Input/IMC_Default.IMC_Default" 0 (struct))))
          (:`CastFailed`
            (`KismetSystemLibrary.PrintString` "GameState캐스팅 안 됨!!!" true true (struct :`R` 1.0 :`B` 0.032277 :`A` 1.0) 5.0))))
      (:`then_1`
        (bind _returnvalue_2 (`|CreateWidget` "/Game/Blueprints/UI/WBP_RoleSelect.WBP_RoleSelect_C"))
        (bind _output_get (set `self.RoleSelectWidgetRef` _returnvalue_2))
        (`UserWidget.AddToViewport` _output_get 0)
        (`WidgetBlueprintLibrary.SetInputMode_UIOnlyEx` _returnvalue null)
        (set `PlayerController.bShowMouseCursor` true _returnvalue)))))

(event `C2S_SelectedRole`
  (params (RequestedRole :type "/Game/Blueprints/Lobby/E_PlayerRole Enum" :default "NewEnumerator0"))
  (if (`self.IsLocalController`)
    (switch `/Game/Blueprints/Lobby/E_PlayerRole` RequestedRole
      (:`NewEnumerator1`
        (if (not (`/Game/Blueprints/Lobby/BP_GameState.bIsHunterTaken` (`self.GameStateRef`)))
          (set `/Game/Blueprints/Lobby/BP_GameState.bIsHunterTaken` true (`self.GameStateRef`))
          (bind _asbp_player_state (cast `/Game/Blueprints/Lobby/BP_PlayerState` (`self.PlayerState`)))
          (set `/Game/Blueprints/Lobby/BP_PlayerState.SelectedRole` (`self.RequestRole`) _asbp_player_state)
          (`self.S2C_SelectedRoleSuccess`)
          (else
            (`KismetSystemLibrary.PrintString` "이미 선택된 역할입니다." true true (struct :`R` 1.0 :`A` 1.0) 5.0))))
      (:`NewEnumerator2`
        (if (not (`/Game/Blueprints/Lobby/BP_GameState.bIsSurvivorTaken` (`self.GameStateRef`)))
          (set `/Game/Blueprints/Lobby/BP_GameState.bIsSurvivorTaken` true (`self.GameStateRef`))
          (bind _asbp_player_state_2 (cast `/Game/Blueprints/Lobby/BP_PlayerState` (`self.PlayerState`)))
          (set `/Game/Blueprints/Lobby/BP_PlayerState.SelectedRole` (`self.RequestRole`) _asbp_player_state_2)
          (`self.S2C_SelectedRoleSuccess`)
          (else
            (`KismetSystemLibrary.PrintString` "이미 선택된 역할입니다." true true (struct :`R` 1.0 :`A` 1.0) 5.0)))))))

(event `S2C_SelectedRoleSuccess`
  (bind _returnvalue (`|CreateWidget` "/Game/Blueprints/UI/WBP_Lobby.WBP_Lobby_C"))
  (`UserWidget.AddToViewport` _returnvalue 0))

(event `S2C_ShowWaitingWidget`
  (bind _returnvalue (`|CreateWidget` "/Game/Blueprints/UI/WBP_Waiting.WBP_Waiting_C"))
  (`UserWidget.AddToViewport` _returnvalue 0))

(fn `UserConstructionScript`)